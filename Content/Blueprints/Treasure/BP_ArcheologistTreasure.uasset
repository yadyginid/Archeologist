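; A draggable treasure sprite that the player drops onto the drop zone to add to the archeologist pawn's gold count.
; Clicking the sprite opens a Gate on Tick that snaps the actor to the cursor's Visibility trace hit point.
; On release, it returns to its start position if BP_DropZone is not ready; otherwise it increments the count and destroys itself.
; Its destruction unblocks the referenced archeologist slot.
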(event OnClicked(PaperSprite)
  (params (TouchedComponent :type Primitive%20Component%20Object%20Reference) (ButtonPressed :type Key%20Structure :default "None"))
  (Utilities|FlowControl|Gate true) ; enters at Open
)

(event OnReleased(PaperSprite)
  (params (TouchedComponent :type Primitive%20Component%20Object%20Reference) (ButtonReleased :type Key%20Structure :default "None"))
  (if (not (Variables|/Game/Blueprints/Drop/BP_DropZone.BP_DropZone_C|GetIsReadyDrop (Variables|Default|GetBP_DropZone)))
    (Transformation|SetActorLocation (Variables|Default|GetInitActorLocation) false false)
    (Utilities|FlowControl|Gate true) ; enters at Close
    (else
      (bind _asbp_archeologist_pawn (Utilities|Casting|CastToBP_ArcheologistPawn (Pawn|GetControlledPawn (Game|GetPlayerController 0))))
      (Utilities|IsValid _asbp_archeologist_pawn
        (:Is%20Valid
          (Class|ArcheologistPawn|IncrCountGolds _asbp_archeologist_pawn)
          (Actor|DestroyActor))))))

(event EventBeginPlay
  (Actor|Tick|SetActorTickEnabled true)
  (Variables|Default|SetInitActorLocation (Transformation|GetActorLocation))
  (bind _returnvalue (Actor|GetActorOfClass "/Game/Blueprints/Drop/BP_DropZone.BP_DropZone_C"))
  (Variables|Default|SetBP_DropZone _returnvalue))

(event EventDestroyed
  (bind _returnvalue (Class|ArcheologistTreasure|ArcheologistSlotRefGet))
  (Utilities|IsValid _returnvalue
    (:Is%20Valid
      (Class|ArcheologistSlot|SetBlock _returnvalue false))))

(event EventTick
  (params (DeltaSeconds :type Float%20%28single-precision%29))
  (Utilities|FlowControl|Gate true
    (:Exit
      (Transformation|SetActorLocation (.Location (Collision|BreakHitResult (.HitResult (Game|Player|GetHitResultUnderCursorbyChannel (Game|GetPlayerController 0) "TraceTypeQuery1" true)))) false false))))

(fn ConstructionScript)