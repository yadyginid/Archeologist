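; Game mode for the Archeologist digging game that handles saving, loading, restarting and the end-of-game screen.
; On BeginPlay it loads the "Save1" slot or creates a new save object, respawning saved treasures and restoring each slot's depth and block state plus the player's gold and shovel counts.
; Restart deletes the save and reopens the level, while ShowResult opens WBP_Menu with a win or game over text.
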(event EventBeginPlay
  (CallFunction|Load))

(event EventShowResult
  (Input|SetInputModeUIOnly (Game|GetPlayerController 0) 0 "DoNotLock")
  (if (Variables|Default|GetPawnWin)
    (Variables|Default|SetTextForEndGame "Game Win")
    (else
      (Variables|Default|SetTextForEndGame "Game Over")))
  (bind _returnvalue (UserInterface|CreateWidget "/Game/UI/WBP_Menu.WBP_Menu_C"))
  (UserInterface|Viewport|AddtoViewport _returnvalue 0)
  (Variables|/Game/UI/WBP_Menu.WBP_Menu_C|SetTextResult _returnvalue (Variables|Default|GetTextForEndGame))
  (Widget|SetVisibility (Variables|/Game/UI/WBP_Menu.WBP_Menu_C|GetGameResultText _returnvalue) "Visible"))

(fn ConstructionScript)

(fn Save
  (CallFunction|ClearSaveDATA)
  (CallFunction|SaveTreasure)
  (CallFunction|SaveSlot)
  (CallFunction|SavePlayer)
  (SaveGame|SaveGametoSlot (Variables|Default|GetBP_ArcheologistSaveGameRef) "Save1"))

(fn Load
  (bind _returnvalue (SaveGame|DoesSaveGameExist "Save1"))
  (if _returnvalue
    (bind _returnvalue_2 (SaveGame|LoadGamefromSlot "Save1"))
    (bind _asbp_archeologist_save_game (Utilities|Casting|CastToBP_ArcheologistSaveGame _returnvalue_2))
    (Variables|Default|SetBP_ArcheologistSaveGameRef _asbp_archeologist_save_game)
    (CallFunction|LoadTreasure)
    (CallFunction|LoadSlot)
    (CallFunction|LoadPlayer)
    (else
      (bind _returnvalue_3 (SaveGame|CreateSaveGameObject "/Game/Blueprints/SaveGame/BP_ArcheologistSaveGame.BP_ArcheologistSaveGame_C"))
      (Variables|Default|SetBP_ArcheologistSaveGameRef _returnvalue_3))))

(fn Restart
  (SaveGame|DeleteGameinSlot "Save1")
  (bind _returnvalue (Game|GetCurrentLevelName true))
  (Game|OpenLevel(byName) (Utilities|String|StringToName _returnvalue)))

(fn SaveTreasure
  (bind _outactors (Actor|GetAllActorsOfClass "/Game/Blueprints/Treasure/BP_ArcheologistTreasure.BP_ArcheologistTreasure_C"))
  (for _array_element _outactors
    (Utilities|Array|Add (Variables|/Game/Blueprints/SaveGame/BP_ArcheologistSaveGame.BP_ArcheologistSaveGame_C|GetSaveTreasure (Variables|Default|GetBP_ArcheologistSaveGameRef)) (Utilities|Struct|MakeS_SaveArrTreasure (Utilities|Struct|MakeS_SaveTreasure (Utilities|GetClass _array_element) (Transformation|GetActorTransform _array_element))))))

(fn ClearSaveDATA
  (Utilities|Array|Clear (Variables|/Game/Blueprints/SaveGame/BP_ArcheologistSaveGame.BP_ArcheologistSaveGame_C|GetSaveTreasure (Variables|Default|GetBP_ArcheologistSaveGameRef)))
  (Utilities|Array|Clear (Variables|/Game/Blueprints/SaveGame/BP_ArcheologistSaveGame.BP_ArcheologistSaveGame_C|GetSaveSlot (Variables|Default|GetBP_ArcheologistSaveGameRef))))

(fn LoadTreasure
  (bind _outactors (Actor|GetAllActorsOfClass "/Game/Blueprints/Treasure/BP_ArcheologistTreasure.BP_ArcheologistTreasure_C"))
  (for _array_element _outactors
    (Actor|DestroyActor _array_element))
  (for _array_element_2 (Variables|/Game/Blueprints/SaveGame/BP_ArcheologistSaveGame.BP_ArcheologistSaveGame_C|GetSaveTreasure (Variables|Default|GetBP_ArcheologistSaveGameRef))
    (Game|SpawnActorfromClass (.class (Utilities|Struct|BreakS_SaveArrTreasure _array_element_2)) (.transform (Utilities|Struct|BreakS_SaveArrTreasure _array_element_2)) "Undefined" 0 0)))

(fn SaveSlot
  (bind _outactors (Actor|GetAllActorsOfClass "/Game/Blueprints/Slot/BP_ArcheologistSlot.BP_ArcheologistSlot_C"))
  (for _array_element _outactors
    (Utilities|Array|Add (Variables|/Game/Blueprints/SaveGame/BP_ArcheologistSaveGame.BP_ArcheologistSaveGame_C|GetSaveSlot (Variables|Default|GetBP_ArcheologistSaveGameRef)) (Utilities|Struct|MakeS_Slot _array_element (Class|ArcheologistSlot|GetDeep _array_element) (Class|ArcheologistSlot|GetBlock _array_element)))))

(fn LoadSlot
  (for _array_element (Variables|/Game/Blueprints/SaveGame/BP_ArcheologistSaveGame.BP_ArcheologistSaveGame_C|GetSaveSlot (Variables|Default|GetBP_ArcheologistSaveGameRef))
    (Class|ArcheologistSlot|SetDeep (.SlotRef (Utilities|Struct|BreakS_Slot _array_element)) (.Deep (Utilities|Struct|BreakS_Slot _array_element)))
    (Class|ArcheologistSlot|SetBlock (.SlotRef (Utilities|Struct|BreakS_Slot _array_element)) (.Block (Utilities|Struct|BreakS_Slot _array_element)))))

(fn SavePlayer
  (bind _asbp_archeologist_pawn (Utilities|Casting|CastToBP_ArcheologistPawn (Game|Player|GetPlayerPawn 0)))
  (Variables|/Game/Blueprints/SaveGame/BP_ArcheologistSaveGame.BP_ArcheologistSaveGame_C|SetSavePlayer (Variables|Default|GetBP_ArcheologistSaveGameRef) (Utilities|Struct|MakeS_PlayerStat (Variables|/Script/Archeologist.ArcheologistPawn|GetCurrentCountGolds _asbp_archeologist_pawn) (Variables|/Script/Archeologist.ArcheologistPawn|GetCurrentCountShovels _asbp_archeologist_pawn))))

(fn LoadPlayer
  (bind _bp_archeologistsavegameref (Variables|Default|GetBP_ArcheologistSaveGameRef))
  (bind _saveplayer (Variables|/Game/Blueprints/SaveGame/BP_ArcheologistSaveGame.BP_ArcheologistSaveGame_C|GetSavePlayer _bp_archeologistsavegameref))
  (bind (_countgolds _countshovels) (Utilities|Struct|BreakS_PlayerStat _saveplayer))
  (bind _asbp_archeologist_pawn (Utilities|Casting|CastToBP_ArcheologistPawn (Game|Player|GetPlayerPawn 0)))
  (Variables|/Script/Archeologist.ArcheologistPawn|SetCurrentCountGolds _asbp_archeologist_pawn _countgolds)
  (Variables|/Script/Archeologist.ArcheologistPawn|SetCurrentCountShovels _asbp_archeologist_pawn _countshovels))